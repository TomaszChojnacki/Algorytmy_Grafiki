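; World actor that generates procedural terrain tiles around the player on a looping timer and spawns lake water and a set element at start.
; GeneratedTiles records built tiles; each new one becomes a collidable procedural mesh section shaped by three octaves of multiplied 1D Perlin noise.
; GetSubset trims a padded vertex border after computing normals and tangents, keeping tile seams smooth.
; Height bands randomly scatter grass, tree and rock HISM instances on vertices.
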(event `self.ReceiveBeginPlay`
  (`|SpawnActorFromClass` "/Game/WaterPlane/Lake/Blueprint/BP_LakeWater.BP_LakeWater_C" (`KismetMathLibrary.MakeTransform` (0.0 0.0 -900.0) (struct) (0.0 0.0 0.0)) "Undefined" "MultiplyWithRoot" null null)
  (`self.SpawnTilesAroundPlayer`)
  (`KismetSystemLibrary.K2_SetTimer` null "SpawnTilesAroundPlayer" 0.5 true)
  (`|SpawnActorFromClass` "/Game/World/BP_ProceduralSetElement.BP_ProceduralSetElement_C" (`KismetMathLibrary.MakeTransform` (-54530.0 -53310.0 0.2)) "Undefined" "MultiplyWithRoot" null null))

(event `SpawnTilesAroundPlayer`
  (bind (_xstart _xend _ystart _yend) (`self.GetTilesAroundPlayer`))
  (for _index (range _ystart (+ _yend 1))
    (for _index_2 (range _xstart (+ _xend 1))
      (`self.Generate` _index_2 _index))))

(fn `Generate`
  (params (SectionIndexX :type Integer) (SectionIndexY :type Integer))
  (locals (UV0L :type "Array of Vector2D Structure") (TrianglesL :type "Array of Integer") (VerticesL :type "Array of Vector Structure") (Offset :type "Vector Structure"))
  (bind _returnvalue (`KismetMathLibrary.RandomFloatInRange` 10.0 25.0))
  (bind _returnvalue_2 (`KismetMathLibrary.RandomFloatInRange` 10.0 12.0))
  (bind _size (`self.Size`))
  (bind _generatedtiles (`self.GeneratedTiles`))
  (bind _proceduralmesh (`self.ProceduralMesh`))
  (bind _verticesl (`local.VerticesL`))
  (bind _trianglesl (`local.TrianglesL`))
  (bind _trianglesl_2 (`local.TrianglesL`))
  (bind _section_index (`self.Section Index`))
  (bind _verticesl_2 (`local.VerticesL`))
  (bind _size_2 (`self.Size`))
  (bind _verticesl_3 (`local.VerticesL`))
  (bind (_offset_x _offset_y) (`KismetMathLibrary.BreakVector` (`local.Offset`)))
  (bind _returnvalue_3 (/ (`self.Size`) 100.0))
  (bind _returnvalue_4 (+ (`self.XVerCount`) 2))
  (if (not (`.ReturnValue` (`BlueprintMapLibrary.Map_Find` _generatedtiles (make `IntPoint` SectionIndexX SectionIndexY))))
    (`BlueprintMapLibrary.Map_Add` _generatedtiles (make `IntPoint` SectionIndexX SectionIndexY) (`self.Section Index`))
    (set `local.Offset` (`KismetMathLibrary.MakeVector` (`KismetMathLibrary.Conv_IntToDouble` (* (`local.SectionIndexX`) (* (- (`self.XVerCount`) 1) _size))) (`KismetMathLibrary.Conv_IntToDouble` (* (`local.SectionIndexY`) (* (- (`self.YVerCount`) 1) _size)))))
    (set `self.Seed` (`KismetMathLibrary.RandomFloatInRange` -10000.0 10000.0))
    (for _index (range -1 (+ (`self.YVerCount`) 1))
      (for _index_2 (range -1 (+ (`self.XVerCount`) 1))
        (bind _returnvalue_5 (+ _offset_x (* _index_2 _size_2)))
        (bind _returnvalue_6 (+ _offset_y (* _index _size_2)))
        (`KismetArrayLibrary.Array_Add` (`local.VerticesL`) (`KismetMathLibrary.MakeVector` _returnvalue_5 _returnvalue_6 (`self.Hight` _returnvalue_5 _returnvalue_6)))
        (`KismetArrayLibrary.Array_Add` (`local.UV0L`) (`KismetMathLibrary.MakeVector2D` (* _returnvalue_3 (`KismetMathLibrary.Conv_IntToDouble` (+ _index (* (`local.SectionIndexX`) (- (`self.XVerCount`) 1))))) (* _returnvalue_3 (`KismetMathLibrary.Conv_IntToDouble` (+ _index_2 (* (`local.SectionIndexY`) (- (`self.YVerCount`) 1)))))))
        (if (`self.Showdebug`)
          (`KismetSystemLibrary.DrawDebugBox` (`KismetMathLibrary.MakeVector` _returnvalue_5 _returnvalue_6) (2.0 2.0 2.0) (struct :`R` 1.0 :`B` 0.008266 :`A` 1.0) (struct) 100.0 2.0))))
    ; Tworzenie trójkątów
    (for _index_3 (range (+ (`self.YVerCount`) 1))
      (for _index_4 (range (+ (`self.XVerCount`) 1))
        (bind _returnvalue_7 (+ _index_4 (* _index_3 _returnvalue_4)))
        (`KismetArrayLibrary.Array_Add` _trianglesl _returnvalue_7)
        (bind _returnvalue_8 (+ _returnvalue_7 _returnvalue_4))
        (`KismetArrayLibrary.Array_Add` _trianglesl _returnvalue_8)
        (bind _returnvalue_9 (+ _returnvalue_7 1))
        (`KismetArrayLibrary.Array_Add` _trianglesl _returnvalue_9)
        (`KismetArrayLibrary.Array_Add` _trianglesl_2 _returnvalue_8)
        (`KismetArrayLibrary.Array_Add` _trianglesl_2 (+ _returnvalue_8 1))
        (`KismetArrayLibrary.Array_Add` _trianglesl_2 _returnvalue_9)
        (if (`self.Showdebug`)
          (bind _output (`|GetArrayItem` (`local.VerticesL`) _returnvalue_9))
          (`KismetSystemLibrary.DrawDebugLine` _output (+ _output (0.0 0.0 10.0)) (struct :`A` 1.0) 100.0 2.0))))
    ; Mesh proceduralny
    (bind (_verticesout _trianglesout _normalsout _uv0lout _tangentsout) (`self.GetSubset` (`local.VerticesL`) (`local.TrianglesL`) (`local.UV0L`)))
    (`ProceduralMeshComponent.CreateMeshSection_LinearColor` :`self` _proceduralmesh :`SectionIndex` _section_index :`Vertices` _verticesout :`Triangles` _trianglesout :`Normals` _normalsout :`UV0` _uv0lout :`Tangents` _tangentsout :`bCreateCollision` true)
    (`PrimitiveComponent.SetMaterial` _proceduralmesh _section_index "/Game/World/Test_Inst.Test_Inst")
    (`/Engine/EditorBlueprintResources/StandardMacros.IncrementInt` (`self.Section Index`)
      (:`  `
        ; Drzewo
        (for (_array_element _array_index) _verticesl
          (bind _returnvalue_10 (`KismetMathLibrary.Dot_VectorVector` (`|GetArrayItem` _verticesl _array_index) (0.0 0.0 1.0)))
          (if (> _returnvalue_10 30.0)
            (if (< _returnvalue_10 100.0)
              (if (< (`KismetMathLibrary.RandomFloatInRange` 0.0 1.0) 0.4)
                (`InstancedStaticMeshComponent.AddInstance` (`self.HISM_Tree`) (`KismetMathLibrary.MakeTransform` _array_element (struct) (`KismetMathLibrary.MakeVector` 1.0 1.0 (`KismetMathLibrary.RandomFloatInRange` 0.5 1.2))) false)))))
        ; Trawa
        (for (_array_element_2 _array_index_2) _verticesl_3
          (bind _returnvalue_11 (`KismetMathLibrary.Dot_VectorVector` (`|GetArrayItem` _verticesl_3 _array_index_2) (0.0 0.0 1.0)))
          (if (> _returnvalue_11 0.0)
            (if (< _returnvalue_11 30.0)
              (if (< (`KismetMathLibrary.RandomFloatInRange` 0.0 1.0) 0.7)
                (`InstancedStaticMeshComponent.AddInstance` (`self.HISM_Grass`) (`KismetMathLibrary.MakeTransform` _array_element_2 (struct) (`KismetMathLibrary.MakeVector` _returnvalue_2 _returnvalue_2 _returnvalue_2)) false)))))
        ; Kamienie
        (for (_array_element_3 _array_index_3) _verticesl_2
          (bind _returnvalue_12 (`KismetMathLibrary.Dot_VectorVector` (`|GetArrayItem` _verticesl_2 _array_index_3) (0.0 0.0 1.0)))
          (if (> _returnvalue_12 101.0)
            (if (< _returnvalue_12 150.0)
              (if (< (`KismetMathLibrary.RandomFloatInRange` 0.0 1.0) 0.5)
                (`InstancedStaticMeshComponent.AddInstance` (`self.HISM_Rock`) (`KismetMathLibrary.MakeTransform` _array_element_3 (struct) (`KismetMathLibrary.MakeVector` _returnvalue _returnvalue _returnvalue)) false)))))))))

(fn `GetPlayerPosition`
  (returns (PX :type Integer) (PY :type Integer))
  (bind _returnvalue (`GameplayStatics.GetPlayerCharacter` 0))
  (bind _size (`self.Size`))
  (bind (_returnvalue_x _returnvalue_y) (`KismetMathLibrary.BreakVector` (`self.K2_GetActorLocation` _returnvalue)))
  (`/Engine/EditorBlueprintResources/StandardMacros.IsValid` _returnvalue
    (:`Is Valid`
      (return (`KismetMathLibrary.FTrunc` (/ _returnvalue_x (* _size (+ (`self.XVerCount`) 1)))) (`KismetMathLibrary.FTrunc` (/ _returnvalue_y (* _size (+ (`self.YVerCount`) 1))))))
    (:`Is Not Valid`
      (return 0 0))))

(fn `GetSubset`
  (params (InVertices :type "Array of Vector Structure") (InTriangles :type "Array of Integer") (InUV0L :type "Array of Vector2D Structure"))
  (returns (VerticesOut :type "Array of Vector Structure") (TrianglesOut :type "Array of Integer") (NormalsOut :type "Array of Vector Structure") (UV0LOut :type "Array of Vector2D Structure") (TangentsOut :type "Array of ProcMeshTangent Structure"))
  (locals (VerticesLoc :type "Array of Vector Structure") (TrianglesLoc :type "Array of Integer") (`UV0L Loc` :type "Array of Vector2D Structure") (TangentsLoc :type "Array of ProcMeshTangent Structure") (NormalsLoc :type "Array of Vector Structure") (NormalsBig :type "Array of Vector Structure") (TangentsBig :type "Array of ProcMeshTangent Structure") (IndexLoc :type Integer :default 0))
  (bind _xvercount (`self.XVerCount`))
  (bind _trianglesloc (`local.TrianglesLoc`))
  (bind _trianglesloc_2 (`local.TrianglesLoc`))
  (bind (_normals _tangents) (`KismetProceduralMeshLibrary.CalculateTangentsForMesh` InVertices InTriangles InUV0L))
  (set `local.NormalsBig` _normals)
  (set `local.TangentsBig` _tangents)
  (for _index (range -1 (+ (`self.YVerCount`) 1))
    (for _index_2 (range -1 (+ (`self.XVerCount`) 1))
      (if (and (> _index_2 -1) (< _index_2 (`self.XVerCount`)) (> _index -1) (< _index (`self.YVerCount`)))
        (`KismetArrayLibrary.Array_Add` (`local.VerticesLoc`) (`|GetArrayItem` (`local.InVertices`) (`local.IndexLoc`)))
        (`KismetArrayLibrary.Array_Add` (`local.UV0L Loc`) (`|GetArrayItem` (`local.InUV0L`) (`local.IndexLoc`)))
        (`KismetArrayLibrary.Array_Add` (`local.NormalsLoc`) (`|GetArrayItem` (`local.NormalsBig`) (`local.IndexLoc`)))
        (`KismetArrayLibrary.Array_Add` (`local.TangentsLoc`) (`|GetArrayItem` (`local.TangentsBig`) (`local.IndexLoc`))))
      (`/Engine/EditorBlueprintResources/StandardMacros.IncrementInt` (`local.IndexLoc`))))
  (for _index_3 (range (+ (- (`self.YVerCount`) 2) 1))
    (for _index_4 (range (+ (- (`self.XVerCount`) 2) 1))
      (bind _returnvalue (+ _index_4 (* _index_3 _xvercount)))
      (`KismetArrayLibrary.Array_Add` _trianglesloc _returnvalue)
      (bind _returnvalue_2 (+ _returnvalue _xvercount))
      (`KismetArrayLibrary.Array_Add` _trianglesloc _returnvalue_2)
      (bind _returnvalue_3 (+ _returnvalue 1))
      (`KismetArrayLibrary.Array_Add` _trianglesloc _returnvalue_3)
      (`KismetArrayLibrary.Array_Add` _trianglesloc_2 _returnvalue_2)
      (`KismetArrayLibrary.Array_Add` _trianglesloc_2 (+ _returnvalue_2 1))
      (`KismetArrayLibrary.Array_Add` _trianglesloc_2 _returnvalue_3)
      (if (`self.Showdebug`)
        (bind _output (`|GetArrayItem` (`local.VerticesLoc`) _returnvalue_3))
        (`KismetSystemLibrary.DrawDebugLine` _output (+ _output (0.0 0.0 10.0)) (struct :`A` 1.0) 100.0 2.0))))
  (return (`local.VerticesLoc`) (`local.TrianglesLoc`) (`local.NormalsLoc`) (`local.UV0L Loc`) (`local.TangentsLoc`)))

(fn `GetTilesAroundPlayer`
  (returns (XStart :type Integer) (XEnd :type Integer) (YStart :type Integer) (YEnd :type Integer))
  (bind (_px _py) (`self.GetPlayerPosition`))
  (bind _numofsectionx (`self.NumOfSectionX`))
  (bind _numofsectiony (`self.NumOfSectionY`))
  (bind _returnvalue (- _px (/ _numofsectionx 2)))
  (bind _returnvalue_2 (- _py (/ _numofsectiony 2)))
  (return _returnvalue (+ _returnvalue _numofsectionx -1) _returnvalue_2 (+ _returnvalue_2 _numofsectiony -1)))

(fn `Hight`
  (params (X :type "Float (double-precision)") (Y :type "Float (double-precision)"))
  (returns (ReturnValue :type "Float (double-precision)"))
  (bind _returnvalue (+ Y 0.0))
  (bind _returnvalue_2 (+ X 0.0))
  (return (+ (`self.PerlinNoise2D` _returnvalue_2 _returnvalue 0.0001 17000.0) (`self.PerlinNoise2D` _returnvalue_2 _returnvalue 0.001 500.0) (`self.PerlinNoise2D` _returnvalue_2 _returnvalue 0.01 100.0))))

(fn `PerlinNoise2D`
  (params (InX :type "Float (double-precision)") (InY :type "Float (double-precision)") (InScale :type "Float (double-precision)") (InAmplitude :type "Float (double-precision)"))
  (returns (ReturnValue :type "Float (double-precision)"))
  (return (* (* (`KismetMathLibrary.PerlinNoise1D` (+ (* InX InScale) 0.1)) (`KismetMathLibrary.PerlinNoise1D` (+ (* InY InScale) 0.1))) InAmplitude)))

(fn `UserConstructionScript`)