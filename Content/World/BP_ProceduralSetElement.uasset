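; Procedural settlement actor that scatters buildings at random in its construction script, with the count growing sublinearly with Population.
; The first placement is a church and the second a residential building; the rest are weighted picks of bookshop, street lamp or house.
; Positions skip exact repeats only.
; PlaceObject adds each mesh component, using a vertical trace's world hit Z as its relative height.
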(fn `PlaceObject`
  (params (Relative :type "Vector2D Structure") (Mesh :type "StaticMesh Object Reference") (Scala :type "Float (double-precision)"))
  (bind (_x _y) (`KismetMathLibrary.BreakVector2D` Relative))
  (bind _returnvalue (+ (`self.K2_GetActorLocation`) Relative))
  (bind _outhit (`KismetSystemLibrary.LineTraceSingle` :`Start` (+ _returnvalue (0.0 0.0 99999.0)) :`End` (+ _returnvalue (0.0 0.0 -99999.0)) :`TraceChannel` "TraceTypeQuery1" :`DrawDebugType` "ForDuration" :`DrawTime` 2.0))
  (bind _returnvalue_2 (`|AddComponentByClass` "/Script/Engine.StaticMeshComponent" false (`KismetMathLibrary.MakeTransform` (`KismetMathLibrary.MakeVector` _x _y (.z (`.Location` (`GameplayStatics.BreakHitResult` _outhit)))) (struct) (`KismetMathLibrary.MakeVector` Scala Scala Scala))))
  (`StaticMeshComponent.SetStaticMesh` _returnvalue_2 Mesh))

(fn `UserConstructionScript`
  (locals (TempTile :type "Vector2D Structure"))
  (bind _returnvalue (`KismetMathLibrary.RandomFloatInRange` 0.0 100.0))
  (bind _temptile (`local.TempTile`))
  (bind _temptile_2 (`local.TempTile`))
  (bind _returnvalue_2 (* _temptile (150.0 150.0)))
  (for _index (range (+ (`KismetMathLibrary.FTrunc` (`KismetMathLibrary.MultiplyMultiply_FloatFloat` (`KismetMathLibrary.Conv_IntToDouble` (`self.Population`)) 0.65)) 1))
    (`KismetMathLibrary.Set2D` _temptile_2 (`KismetMathLibrary.RandomFloatInRange` -100.0 120.0) (`KismetMathLibrary.RandomFloatInRange` -100.0 120.0))
    (if (not (`KismetArrayLibrary.Array_Contains` (`self.UsedTiles`) _temptile_2))
      (if (> _index 0)
        (if (>= _index 2)
          (if (and (< _returnvalue 80.0) (> _returnvalue 70.0))
            (`self.PlaceObject` _returnvalue_2 "/Game/Fab/Magic_bookshop/magic_bookshop/StaticMeshes/magic_bookshop.magic_bookshop" 1.7)
            (elif (< (`KismetMathLibrary.RandomFloatInRange` 0.0 100.0) 40.0)
              (`self.PlaceObject` _returnvalue_2 "/Game/Fab/Street_Lamp/street_lamp/StaticMeshes/street_lamp.street_lamp" 1.6)
              (else
                (`self.PlaceObject` _returnvalue_2 "/Game/Fab/American_House/house/StaticMeshes/house.house" 0.8))))
          (else
            (`self.PlaceObject` _returnvalue_2 "/Game/Fab/Residential_building/residential_building/StaticMeshes/residential_building.residential_building" 1.0)))
        (else
          (`self.PlaceObject` _returnvalue_2 "/Game/Fab/Church__Low_Poly_/church_low_poly/StaticMeshes/church_low_poly.church_low_poly" 0.08)))
      (`KismetArrayLibrary.Array_Add` (`self.UsedTiles`) _temptile))))